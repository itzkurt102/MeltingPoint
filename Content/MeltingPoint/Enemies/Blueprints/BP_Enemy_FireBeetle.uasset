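; BP_Enemy_FireBeetle is the fire beetle enemy, with health, player detection, an attack and a floating health bar.
; Pawn sensing sets the hasSeenPlayer blackboard key, while AttackPlayer sphere-traces forward over the aggro range and damages a player it hits.
; Damage reduces health, and at zero the beetle spawns its dead-variant actor and destroys itself.
; Tick refreshes the widget bar and turns it toward the camera; an attack montage is stubbed but unconnected.
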(event OnSeePawn(PawnSensing)
  (params (Pawn :type Pawn%20Object%20Reference))
  ;[1 1 1] Sense Player
  (Utilities|Casting|CastToBP_PlayerCharacter Pawn)
  (AI|Components|Blackboard|SetValueasBool (AI|GetBlackboard (AI|GetAIController self)) (Utilities|Name|MakeLiteralName "hasSeenPlayer") true))

(event Custom|Attack%20Player
  (bind _returnvalue (Transformation|GetActorLocation))
  ;[1 1 1] Attack Player
  (bind (_outhit _returnvalue_2) (Collision|SphereTraceForObjects _returnvalue (+ _returnvalue (* (Math|Vector|GetForwardVector (Transformation|GetActorRotation)) (Variables|Default|GetEnemyAggroRange))) 8e+01 (Utilities|Array|MakeArray "ObjectTypeQuery3") false 0 "None" true "(R=1.000000,G=0.000000,B=0.000000,A=1.000000)" "(R=0.000000,G=1.000000,B=0.000000,A=1.000000)" 1.0))
  (if _returnvalue_2
    (Utilities|Casting|CastToBP_PlayerCharacter (.HitActor (Collision|BreakHitResult _outhit)))
    (Game|Damage|ApplyDamage (.HitActor (Collision|BreakHitResult _outhit)) (Variables|Default|GetFireBeetleDamage) 0 self "/Script/Engine.DamageType")))

(event EventTick
  (params (DeltaSeconds :type Float%20%28single-precision%29))
  (bind _healthbarwidget (Variables|Default|GetHealthBarWidget))
  ;[1 1 1] Enemy Health Bar Update
  (bind _aswb_fire_beetle_health_bar (Utilities|Casting|CastToWB_FireBeetleHealthBar (UserInterface|GetWidget (Variables|Default|GetHealthBarWidget))))
  (Progress|SetPercent (Variables|/Game/MeltingPoint/UI/HealthBars/WB_FireBeetleHealthBar.WB_FireBeetleHealthBar_C|GetFireBeetleHealthBar _aswb_fire_beetle_health_bar) (/ (Variables|Default|GetCurrentHealth) (Variables|Default|GetMaxHealth)))
  (Transformation|SetWorldRotation _healthbarwidget (Math|Rotator|FindLookatRotation (Transformation|GetWorldLocation _healthbarwidget) (Transformation|GetWorldLocation (Variables|/Script/Engine.PlayerCameraManager|GetTransformComponent (Game|GetPlayerCameraManager 0)))) false false))

(event EventBeginPlay
  ;[1 1 1] Set Max Health Variable
  (Variables|Default|SetMaxHealth (Variables|Default|GetCurrentHealth)))

(event Game|Damage|EventAnyDamage
  (params (Damage :type Float%20%28single-precision%29) (DamageType :type Damage%20Type%20Object%20Reference) (InstigatedBy :type Controller%20Object%20Reference) (DamageCauser :type Actor%20Object%20Reference))
  ;[1 1 1] Take Damage
  (bind _output_get (Variables|Default|SetCurrentHealth (- (Variables|Default|GetCurrentHealth) Damage)))
  (if (<= _output_get 0.0)
    (Game|SpawnActorfromClass "/Game/MeltingPoint/Enemies/Blueprints/BP_Enemy_FireBeetle_Dead.BP_Enemy_FireBeetle_Dead_C" (Transformation|GetActorTransform) "AlwaysSpawn" 0 0)
    (Actor|DestroyActor)))

(fn ConstructionScript)