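; Destructible fire beetle nest enemy that periodically spawns fire beetles around itself until it is killed.
; BeginPlay runs a gated retriggerable-delay loop that, while spawning is allowed, places beetles at random offsets until a spawn-count cap is passed.
; Damage drains health; at zero it spawns a dead-nest actor, decrements the player's living-nest count and destroys itself.
; Tick refreshes the health bar widget and turns it toward the camera.
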(event EventTick
  (params (DeltaSeconds :type Float%20%28single-precision%29))
  (bind _healthbarwidget (Variables|Default|GetHealthBarWidget))
  ;[1 1 1] Enemy Health Bar Update
  (bind _aswb_fire_beetle_nest_health_bar (Utilities|Casting|CastToWB_FireBeetleNestHealthBar (UserInterface|GetWidget (Variables|Default|GetHealthBarWidget))))
  (Progress|SetPercent (Variables|/Game/MeltingPoint/UI/HealthBars/WB_FireBeetleNestHealthBar.WB_FireBeetleNestHealthBar_C|GetFireBeetleHealthBar _aswb_fire_beetle_nest_health_bar) (/ (Variables|Default|GetCurrentHealth) (Variables|Default|GetMaxHealth)))
  (Transformation|SetWorldRotation _healthbarwidget (Math|Rotator|FindLookatRotation (Transformation|GetWorldLocation _healthbarwidget) (Transformation|GetWorldLocation (Variables|/Script/Engine.PlayerCameraManager|GetTransformComponent (Game|GetPlayerCameraManager 0)))) false false))

(event EventBeginPlay
  ;[1 1 1] Set Max Health Variable
  (if (Variables|Default|GetcanSpawnFireBeetle) :!label _label
    (Utilities|FlowControl|Sequence
      (:then_0
        (goto _label_2 Open))
      (:then_1
        (Utilities|FlowControl|Gate true :!label _label_2
          (:Exit
            (Utilities|FlowControl|Sequence
              (:then_0
                (CallFunction|SpawnFireBeetle))
              (:then_1
                (Utilities|FlowControl|RetriggerableDelay (Variables|Default|GetTimeBetweenSpawns))
                (goto _label)))))))
    (else
      (goto _label_2 Close))))

(event Game|Damage|EventAnyDamage
  (params (Damage :type Float%20%28single-precision%29) (DamageType :type Damage%20Type%20Object%20Reference) (InstigatedBy :type Controller%20Object%20Reference) (DamageCauser :type Actor%20Object%20Reference))
  ;[1 1 1] Take Damage
  (bind _output_get (Variables|Default|SetCurrentHealth (- (Variables|Default|GetCurrentHealth) Damage)))
  (if (<= _output_get 0.0)
    (Game|SpawnActorfromClass "/Game/MeltingPoint/Enemies/Blueprints/BP_FireBeetleNestDead.BP_FireBeetleNestDead_C" (Transformation|GetActorTransform) "AlwaysSpawn" 0 0)
    (bind _asbp_player_character (Utilities|Casting|CastToBP_PlayerCharacter (Game|GetPlayerCharacter 0)))
    (Variables|/Game/MeltingPoint/Character/Blueprints/BP_PlayerCharacter.BP_PlayerCharacter_C|SetnumAliveNests _asbp_player_character (- (Variables|/Game/MeltingPoint/Character/Blueprints/BP_PlayerCharacter.BP_PlayerCharacter_C|GetnumAliveNests _asbp_player_character) 1.0))
    (Actor|DestroyActor)))

(fn ConstructionScript)

(fn SpawnFireBeetle
  (bind _returnvalue (Transformation|GetActorTransform))
  (bind _returnvalue_2 (Math|Random|RandomFloatinRange 6e+02 1e+03))
  ;[1 1 1] Spawn Fire Beetle
  (if (<= (Variables|Default|GetNumFireBeetlesSpawned) (Variables|Default|GetMaxFireBeetlesSpawned))
    (Game|SpawnActorfromClass "/Game/MeltingPoint/Enemies/Blueprints/BP_Enemy_FireBeetle.BP_Enemy_FireBeetle_C" (Math|Transform|MakeTransform (Math|Vector|MakeVector (+ (.x (.location _returnvalue)) _returnvalue_2) (+ (.y (.location _returnvalue)) _returnvalue_2) (+ (.z (.location _returnvalue)) 5.0)) "0, 0, 0" "1.000000,1.000000,1.000000") "AlwaysSpawn" 0 0)
    (Variables|Default|SetNumFireBeetlesSpawned (+ (Variables|Default|GetNumFireBeetlesSpawned) 1.0))))